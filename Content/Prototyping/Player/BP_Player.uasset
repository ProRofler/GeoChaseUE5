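; Prototype player Blueprint for GeoChase that handles a random body color, a throw action and chase target switching.
; On BeginPlay the authority rolls PlayerColor, and its RepNotify applies it through a lazily created dynamic material instance on the mesh.
; Left click sends a server action that passes the player controller to the GeoChase game state's TryAction.
; R calls NextChaseTarget when the game state allows actions.
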(event Custom|Server_Action
  ;[0.4499 0.8278 1] Throw logic
  (bind _asbp_geo_chase_game_state (Utilities|Casting|CastToBP_GeoChaseGameState (Game|GetGameState)))
  (Class|GCGameStateBase|TryAction _asbp_geo_chase_game_state (.AsPlayer%20Controller (Utilities|Casting|CastToPlayerController (Pawn|GetController)))))

(event Custom|Server_SetPlayerColor
  ;[1 0.5501 0.8664] Random player color
  (Variables|Default|SetPlayerColor (Utilities|Struct|MakeLinearColor (Math|Random|RandomFloat) (Math|Random|RandomFloat) (Math|Random|RandomFloat) 1.0)))

(event EventBeginPlay
  ;[1 0.5501 0.8664] Random player color
  (if (Ability|HasAuthority)
    (CallFunction|ServerSetPlayerColor)))

(event Collision|EventActorBeginOverlap
  (params (OtherActor :type Actor%20Object%20Reference)))

(event EventTick
  (params (DeltaSeconds :type Float%20%28single-precision%29)))

(event Input|KeyboardEvents|R
  (params (Key :type Key%20Structure :default "None"))
  ;[0.4218 0.5312 1] Chase Target Switch Logic
  (:Pressed
    (bind _asbp_geo_chase_game_state (Utilities|Casting|CastToBP_GeoChaseGameState (Game|GetGameState)))
    (if (Class|GCGameStateBase|GetCanDoAction _asbp_geo_chase_game_state)
      (Class|GCPlayerInterface|NextChaseTarget))))

(event Input|MouseEvents|LeftMouseButton
  (params (Key :type Key%20Structure :default "None"))
  ;[0.4499 0.8278 1] Throw logic
  (:Pressed
    (CallFunction|ServerAction)))

(fn ConstructionScript)

(fn OnRepPlayerColor
  (Variables|Default|GetMI_BodyRandom
    (:then
      _)
    (:else
      (bind _returnvalue (CallFunction|CreateDynMat))
      (Variables|Default|SetMI_BodyRandom _returnvalue)))
  (Rendering|Material|SetVectorParameterValue (Variables|Default|GetMI_BodyRandom) "BodyColor" (Variables|Default|GetPlayerColor) :!class /Script/Engine.MaterialInstanceDynamic))

(fn CreateDynMat
  (bind _returnvalue (Rendering|Material|CreateDynamicMaterialInstance (Utilities|Array|Get(acopy) (Rendering|Material|GetMaterials (Variables|Character|GetMesh))) "MI_BodyRandom" "None" :!class /Script/Engine.KismetMaterialLibrary))
  (Rendering|Material|SetMaterial (Variables|Character|GetMesh) 0 _returnvalue)
  (return _returnvalue))