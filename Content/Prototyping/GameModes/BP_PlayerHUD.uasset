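; BP_PlayerHUD manages the prototype's in-game and end-of-session screens for the local player.
; On BeginPlay it creates WBP_Main and a collapsed WBP_End, then binds to the GCGameStateBase session-ended event.
; When the session ends it swaps the widgets, shows the cursor and switches to UI-only input.
; The end screen shows the top leaderboard entry's name and score, or a draw message if there is no leader.
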(event Custom|OnSessionEnded
  (bind _returnvalue (Class|GameplayStatics|GetPlayerControllerfromID))
  (bind _as_gcgame_state_base (Variables|Default|GetAs%20GCGame%20State%20Base))
  (bind _returnvalue_2 (Class|GCGameStateBase|GetLeaderboard _as_gcgame_state_base))
  (bind _output (Utilities|Array|Get(acopy) _returnvalue_2))
  (bind (_name _score) (Utilities|Struct|BreakGCLeaderboardData _output))
  (Widget|SetVisibility (Variables|Default|GetEndWidget) "Visible")
  (Widget|SetVisibility (Variables|Default|GetMainWidget) "Collapsed")
  (Variables|/Script/Engine.PlayerController|SetbShowMouseCursor _returnvalue true)
  (Input|SetInputModeUIOnly _returnvalue (Variables|Default|GetEndWidget) "DoNotLock" false)
  (if (Class|GCGameStateBase|DoesHaveLeader (Variables|Default|GetAs%20GCGame%20State%20Base))
    (Default|SetWinner (Variables|Default|GetEndWidget) (Utilities|Text|ToText(String) (Utilities|String|MakeLiteralString (Utilities|String|Append (Utilities|String|ToString(Name) _name) " score: " (Utilities|String|ToString(Integer) _score)))))
    (else
      (Default|SetWinner (Variables|Default|GetEndWidget) "Roud draw"))))

(event EventBeginPlay
  (bind _asgcgame_state_base (Utilities|Casting|CastToGCGameStateBase (Game|GetGameState)))
  (Variables|Default|SetAs%20GCGame%20State%20Base _asgcgame_state_base)
  (bind _returnvalue (UserInterface|CreateWidget "/Game/Prototyping/UI/Game/WBP_Main.WBP_Main_C" (Class|GameplayStatics|GetPlayerControllerfromID)))
  (bind _output_get (Variables|Default|SetMainWidget _returnvalue))
  (UserInterface|Viewport|AddtoViewport _output_get 0)
  (bind _returnvalue_2 (UserInterface|CreateWidget "/Game/Prototyping/UI/WBP_End.WBP_End_C" (Class|GameplayStatics|GetPlayerControllerfromID)))
  (bind _output_get_2 (Variables|Default|SetEndWidget _returnvalue_2))
  (UserInterface|Viewport|AddtoViewport _output_get_2 0)
  (Widget|SetVisibility (Variables|Default|GetEndWidget) "Collapsed")
  (EventDispatchers|BindEventtoOnSessionEnded (Variables|Default|GetAs%20GCGame%20State%20Base) (EventDispatchers|CreateEvent :!event Custom|OnSessionEnded)))

(event Collision|EventActorBeginOverlap
  (params (OtherActor :type Actor%20Object%20Reference)))

(event EventTick
  (params (DeltaSeconds :type Float%20%28single-precision%29)))

(fn ConstructionScript)