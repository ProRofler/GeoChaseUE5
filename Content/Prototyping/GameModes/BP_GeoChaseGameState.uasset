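; Prototype game state for the GeoChase mode that reacts to session end and picks a losing NPC during the chase.
; BeginPlay binds to the session-ended and can-do-action-changed events; ending the session prints a game-over message.
; When the action flag turns false, the server flags the NPC furthest from the chase target as loser and stops it, retrying next tick if no target exists.
; Debug leaderboard and loser printouts exist but are disconnected.
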(event Custom|EndSession
  (Development|PrintString "Game OVER" true false "(R=1.000000,G=0.000000,B=0.047202,A=1.000000)")
  (if (Ability|HasAuthority)
    _))

(event Custom|FindLoser
  (params (NewValue :type Boolean))
  ;[1 0.9529 0.08412] Handle loser NPC
  (if (and (not NewValue) (Ability|HasAuthority))
    (Utilities|FlowControl|DelayUntilNextTick)
    (bind _outactors (Actor|GetAllActorsOfClass "/Game/Prototyping/NPC/BP_NPC.BP_NPC_C"))
    (bind _returnvalue (Actor|GetActorOfClass "/Script/GeoChase.GCChaseTargetBase"))
    (Utilities|IsValid _returnvalue
      (:Is%20Valid
        (Utilities|IsValid (Class|GCGameStateBase|FindFurthestActor (Transformation|GetActorLocation _returnvalue) _outactors)
          (:Is%20Valid
            (Utilities|IsValid (AI|GetAIController (Class|GCGameStateBase|FindFurthestActor (Transformation|GetActorLocation _returnvalue) _outactors))
              (:Is%20Valid
                (bind _asbp_aicontroller (Utilities|Casting|CastToBP_AIController (AI|GetAIController (Class|GCGameStateBase|FindFurthestActor (Transformation|GetActorLocation _returnvalue) _outactors))))
                (Variables|/Game/Prototyping/NPC/BP_AIController.BP_AIController_C|SetAmIALoser _asbp_aicontroller true)
                (AI|Navigation|StopMovement _asbp_aicontroller))))))
      (:Is%20Not%20Valid
        (CallFunction|FindLoser false)))))

(event EventBeginPlay
  (EventDispatchers|BindEventtoOnSessionEnded (EventDispatchers|CreateEvent :!event Custom|EndSession))
  (EventDispatchers|BindEventtoOnCanDoActionChanged (EventDispatchers|CreateEvent :!event Custom|FindLoser)))

(event EventTick
  (params (DeltaSeconds :type Float%20%28single-precision%29)))

(fn ConstructionScript)