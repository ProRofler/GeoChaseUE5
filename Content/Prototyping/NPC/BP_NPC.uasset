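; BP_NPC is a prototype NPC with a CharacterMovement component and a text render that displays its NameID.
; On BeginPlay, the authority gives it a random max walk speed.
; It then waits a tick, plus one more if NameID is still None, so the name can be assigned before the label text is set.
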(event EventBeginPlay
  (bind _nameid (Variables|Default|GetNameID))
  (if (Ability|HasAuthority)
    (Variables|/Script/Engine.CharacterMovementComponent|SetMaxWalkSpeed (Variables|Character|GetCharacterMovement) (Math|Random|RandomFloatinRange 3e+02 1.2e+03)))
  (Utilities|FlowControl|DelayUntilNextTick) ; It's that or call for super after name assigned
  (if (== _nameid "")
    (Utilities|FlowControl|DelayUntilNextTick) ; It's that or call for super after name assigned
  )
  (Rendering|Components|TextRender|SetText (Variables|Default|GetTextRender) (Utilities|Text|ToText(Name) _nameid)))

(event Collision|EventActorBeginOverlap
  (params (OtherActor :type Actor%20Object%20Reference)))

(event EventTick
  (params (DeltaSeconds :type Float%20%28single-precision%29)))

(fn ConstructionScript)